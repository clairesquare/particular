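; Manager that drives a Niagara particle system's total count and color mix, and sets the player's starting weight class from the dominant color.
; Manage_Particles raises the chosen color's share and lowers the least recently raised one, using counter-stamped ages and re-stamping any color that hits zero.
; AdjustTotalParticles applies clamped pickup changes and opens a Tick gate that steadily drains the count until it reaches the minimum.
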(event `self.ReceiveBeginPlay`
  (bind _niagaracomponent (`NiagaraActor.NiagaraComponent` (`self.Niagara_Actor`)))
  (`NiagaraComponent.SetNiagaraVariableFloat` _niagaracomponent "User.TotalSR" (`self.TotalNbParticles`))
  (for (_array_element _array_index) (`self.Colors_SR_Array`)
    (`NiagaraComponent.SetNiagaraVariableFloat` _niagaracomponent (`|GetArrayItem` (`self.Niagara_User.Colors_Array`) _array_index) _array_element))
  ;[0 0 0] RK- Let our player character know our Starting weight class
  (bind _highest_color_weight_class (`self.Get Highest Current Color Value`))
  (bind _outactors (`GameplayStatics.GetAllActorsOfClass` "/Game/ThirdPersonBP/Blueprints/ThirdPersonCharacter.ThirdPersonCharacter_C"))
  (`/Game/ThirdPersonBP/Blueprints/ThirdPersonCharacter.AdjustSpeedCapByWeight` (`|GetArrayItem` _outactors) _highest_color_weight_class))

(event `Adjust Total Particles`
  (params (NumPArticlesToAdd :type "Float (double-precision)"))
  ;[0 0 0] RK- Functions for decreasing particle count over time and adding/subtracting from current total particles on pickup! (Could be optimized out of tick for later performance gains)
  (bind _output_get (set `self.TotalNbParticles` (`KismetMathLibrary.FClamp` (+ NumPArticlesToAdd (`self.TotalNbParticles`)) (`self.MinNumParticles`) (`self.MaxNumParticles`))))
  (`NiagaraComponent.SetNiagaraVariableFloat` (`NiagaraActor.NiagaraComponent` (`self.Niagara_Actor`)) "User.TotalSR" _output_get) ; This changes value of current num of particles in Niagara,\nall at once. We could make a add a gradual but quick change\ncurrent to desired particle count as well!
  (`self.Begin Particle Loss`) ; Activates decrease below in case\nwe were already at min particles
)

(event `Manage_Particles`
  (params (Particle_Type :type Integer))
  (bind _globalcounter (`self.GlobalCounter`))
  (bind _colors_sr_array (`self.Colors_SR_Array`))
  (bind _globalcounter_2 (`self.GlobalCounter`))
  (bind _indexofminvalue (`self.IndexOfMinValue`))
  (bind _colorindex (`self.ColorIndex`))
  (bind _colors_sr_array_2 (`self.Colors_SR_Array`))
  (bind _indexofminvalue_2 (`KismetMathLibrary.MinOfIntArray` (`self.Colors_Age_Array`)))
  (bind _returnvalue (`KismetMathLibrary.FClamp` (+ (`self.ColorValue2Increase`) (`self.IncrementStep`)) 0.0 100.0))
  (bind _returnvalue_2 (`KismetMathLibrary.FClamp` (- (`self.ColorValue2Decrease`) (`self.IncrementStep`)) 0.0 100.0))
  ;[0 0.01445 1] Zied % incrementer
  (`|ExecutionSequence`
    (:`then_0`
      (set `self.ColorIndex` Particle_Type))
    (:`then_1`
      (set `self.ColorValue2Increase` (`|GetArrayItem` (`self.Colors_SR_Array`) _colorindex))
      (`/Engine/EditorBlueprintResources/StandardMacros.IncrementInt` _globalcounter_2
        (:`  `
          (`KismetArrayLibrary.Array_Set` (`self.Colors_Age_Array`) _colorindex _globalcounter_2)
          (set `self.ColorValue2Decrease` (`|GetArrayItem` (`self.Colors_SR_Array`) _indexofminvalue_2))
          (set `self.IndexOfMinValue` _indexofminvalue_2))))
    (:`then_2`
      (`KismetArrayLibrary.Array_Set` _colors_sr_array_2 _colorindex _returnvalue)
      (`NiagaraComponent.SetNiagaraVariableFloat` (`NiagaraActor.NiagaraComponent` (`self.Niagara_Actor`)) (`|GetArrayItem` (`self.Niagara_User.Colors_Array`) (`self.ColorIndex`)) _returnvalue))
    (:`then_3`
      (`KismetArrayLibrary.Array_Set` _colors_sr_array_2 _indexofminvalue _returnvalue_2)
      (`NiagaraComponent.SetNiagaraVariableFloat` (`NiagaraActor.NiagaraComponent` (`self.Niagara_Actor`)) (`|GetArrayItem` (`self.Niagara_User.Colors_Array`) _indexofminvalue) _returnvalue_2)
      (if (== _returnvalue_2 0.0)
        (`/Engine/EditorBlueprintResources/StandardMacros.IncrementInt` _globalcounter
          (:`  `
            (`KismetArrayLibrary.Array_Set` (`self.Colors_Age_Array`) (`self.IndexOfMinValue`) _globalcounter))))
      (`|ExecutionSequence`
        (:`then_0`
          (`KismetSystemLibrary.PrintString` (`KismetStringLibrary.Conv_DoubleToString` (`|GetArrayItem` _colors_sr_array)) true true (struct :`R` 0.086426 :`G` 0.245707 :`B` 1.0 :`A` 1.0)))
        (:`then_1`
          (`KismetSystemLibrary.PrintString` (`KismetStringLibrary.Conv_DoubleToString` (`|GetArrayItem` _colors_sr_array 1)) true true (struct :`R` 0.912801 :`G` 0.019425 :`B` 0.051565 :`A` 1.0)))
        (:`then_2`
          (`KismetSystemLibrary.PrintString` (`KismetStringLibrary.Conv_DoubleToString` (`|GetArrayItem` _colors_sr_array 2)) true true (struct :`R` 0.052132 :`G` 0.991252 :`B` 0.153853 :`A` 1.0)))))))

(event `self.ReceiveTick`
  (params (DeltaSeconds :type "Float (single-precision)"))
  (bind _totalnbparticles (`self.TotalNbParticles`))
  ;[0 0 0] RK- Functions for decreasing particle count over time and adding/subtracting from current total particles on pickup! (Could be optimized out of tick for later performance gains)
  (`/Engine/EditorBlueprintResources/StandardMacros.Gate` false :!label _label
    (:`Exit`
      (bind _output_get (set `self.TotalNbParticles` (`KismetMathLibrary.FInterpTo_Constant` _totalnbparticles (- _totalnbparticles 10.0) DeltaSeconds (`self.Speed of Particle Loss`))))
      (`NiagaraComponent.SetNiagaraVariableFloat` (`NiagaraActor.NiagaraComponent` (`self.Niagara_Actor`)) "User.TotalSR" _output_get)
      (if (<= _output_get (`self.MinNumParticles`))
        (`self.End Particle Loss`) ; Calls back to red function event earlier, \nstops the decrementer if we reach min particles
      ))))

(event `Begin Particle Loss`
  ;[0 0 0] RK- Functions for decreasing particle count over time and adding/subtracting from current total particles on pickup! (Could be optimized out of tick for later performance gains)
  (goto _label :!via `Open`))

(event `End Particle Loss`
  ;[0 0 0] RK- Functions for decreasing particle count over time and adding/subtracting from current total particles on pickup! (Could be optimized out of tick for later performance gains)
  (goto _label :!via `Close`))

(fn `Get Highest Current Color Value`
  (returns (`Highest Color Weight Class` :type "/Game/BP/ParticleWeightClass_Enum Enum"))
  (bind _indexofmaxvalue (`KismetMathLibrary.MaxOfFloatArray` (`self.Colors_SR_Array`)))
  (if (== _indexofmaxvalue 0)
    (return "NewEnumerator1")
    (elif (== _indexofmaxvalue 1)
      (return "NewEnumerator2")
      (elif (== _indexofmaxvalue 2)
        (return "NewEnumerator0")
        (else
          (return "NewEnumerator3"))))))

(fn `UserConstructionScript`)